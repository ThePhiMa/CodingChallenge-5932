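; BP_ListeningActor is an actor that watches a Buddy reference and reacts to its death.
; On BeginPlay it shows beginning text on its widget, and only the authority starts the WaitForBoolChange async listener on a valid Buddy.
; When the watched bool turns true, it shows ending text, waits briefly, spawns a poof effect at its location and destroys itself.
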(event Custom|CheckForBoolChange
  (bind _buddy (Variables|Default|GetBuddy))
  (Utilities|IsValid _buddy
    (:Is%20Valid
      (bind _bnewvalue (|WaitforBoolChange _buddy)
        (:OnBoolValueChange
          (Development|PrintString "My buddy is dead!" true true "(R=1.000000,G=0.062442,B=0.072389,A=1.000000)")
          (if _bnewvalue
            (CallFunction|OnBuddyDead)))))
    (:Is%20Not%20Valid
      (Development|PrintString "I'm missing my buddy reference!"))))

(event Custom|OnBuddyDead
  (CallFunction|SetWidgetText (Variables|Default|GetText_Ending))
  (Utilities|FlowControl|Delay 2.0)
  (Niagara|SpawnSystematLocation (Variables|Default|GetPoofFX) (Transformation|GetActorLocation))
  (Actor|DestroyActor))

(event EventBeginPlay
  (CallFunction|SetWidgetText (Variables|Default|GetText_Beginning))
  (Networking|SwitchHasAuthority
    (:Authority
      (CallFunction|CheckforBoolChange))))

(fn ConstructionScript)

(fn SetWidgetText
  (params (Text :type Text))
  (bind _astext_widget (Utilities|Casting|CastToTextWidget (UserInterface|GetWidget (Variables|Default|GetTextWidget))))
  (Default|SetText _astext_widget Text)
  (return))