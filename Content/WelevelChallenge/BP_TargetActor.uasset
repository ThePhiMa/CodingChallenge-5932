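; BP_TargetActor is a shootable target that loses life when hit by a WelevelChallengeProjectile and destroys itself when dead.
; Each projectile hit calls LoseLife, then CheckIfDead, which also refreshes the text widget and prints remaining lives before returning the death state.
; The widget shows a random entry from Texts, picked at BeginPlay and on every hit.
; Death prints a message and spawns a PoofFX effect before destroying the actor.
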(event Custom|OnHit
  (Class|TargetActor|LoseLife 25)
  (bind _isdead (CallFunction|CheckifDead))
  (if _isdead
    (CallFunction|OnDead)))

(event Custom|OnDead
  (Development|PrintText "I'm dead xD!")
  (Niagara|SpawnSystematLocation (Variables|Default|GetPoofFX) (Transformation|GetActorLocation))
  (Actor|DestroyActor))

(event EventBeginPlay
  (CallFunction|SetRandomWidgetText))

(event Collision|EventHit
  (params (MyComp :type Primitive%20Component%20Object%20Reference) (Other :type Actor%20Object%20Reference) (OtherComp :type Primitive%20Component%20Object%20Reference) (bSelfMoved :type Boolean) (HitLocation :type Vector :default "0, 0, 0") (HitNormal :type Vector :default "0, 0, 0") (NormalImpulse :type Vector :default "0, 0, 0") (Hit :type Hit%20Result%20Structure%20%28by%20ref%29))
  (if (Utilities|ClassIsChildOf (Utilities|GetClass Other) "/Script/WelevelChallenge.WelevelChallengeProjectile")
    (CallFunction|OnHit)))

(fn ConstructionScript)

(fn CheckifDead
  (CallFunction|SetRandomWidgetText)
  (bind _returnvalue (Class|TargetActor|GetLifesRemaining))
  (Development|PrintText (Utilities|Text|ToText(String) (Utilities|String|Append "Lifes left: " (Utilities|String|ToString(Integer) _returnvalue))))
  (bind _returnvalue_2 (Class|TargetActor|IsDead))
  (return _returnvalue_2))

(fn SetWidgetText
  (params (Text :type Text))
  (bind _astext_widget (Utilities|Casting|CastToTextWidget (UserInterface|GetWidget (Variables|Default|GetTextWidget))))
  (Default|SetText _astext_widget Text)
  (return))

(fn SetRandomWidgetText
  (bind _texts (Variables|Default|GetTexts))
  (CallFunction|SetWidgetText (Utilities|Array|Get(acopy) _texts (Math|Random|RandomIntegerinRange 0 (- (Utilities|Array|Length _texts) 1))))
  (return))